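; Map 03 child of the TD game mode that ends the match with a win or lose screen.
; Tick runs the parent logic, then polls IsVictory and, failing that, IsDefeat.
; Each outcome fires through its own DoOnce, calling the HUD widget's pause-button handler and adding Win_UI or Lose_UI to the viewport for the first player.
; BeginPlay and construction only call the parent.
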(event EventBeginPlay
  (|CallParentFunction))

(event EventTick
  (params (DeltaSeconds :type Float%20%28single-precision%29))
  (|CallParentFunction DeltaSeconds)
  (bind _returnvalue (Class|TDGameMode|IsVictory))
  (if _returnvalue
    (Utilities|FlowControl|DoOnce false
      (:Completed
        (Class|TDHUDWidget|OnPauseButtonClicked (Variables|Default|GetHUDWidget))
        (bind _returnvalue_2 (UserInterface|CreateWidget "/Game/Core/UI/Win_UI.Win_UI_C" (Game|GetPlayerController 0)))
        (UserInterface|Viewport|AddtoViewport _returnvalue_2 0)))
    (else
      (bind _returnvalue_3 (Class|TDGameMode|IsDefeat))
      (if _returnvalue_3
        (Utilities|FlowControl|DoOnce false
          (:Completed
            (Class|TDHUDWidget|OnPauseButtonClicked (Variables|Default|GetHUDWidget))
            (bind _returnvalue_4 (UserInterface|CreateWidget "/Game/Core/UI/Lose_UI.Lose_UI_C" (Game|GetPlayerController 0)))
            (UserInterface|Viewport|AddtoViewport _returnvalue_4 0)))))))

(fn ConstructionScript
  (|CallParentFunction))